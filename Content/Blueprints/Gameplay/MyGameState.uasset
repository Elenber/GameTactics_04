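; Game state that gives players passive coin income and tracks which colors are available.
; On BeginPlay, a looping timer adds one coin to every MyPlayerState in PlayerArray.
; SwitchOffColorEnum updates the given color's slot in AvailableColors, indexed by the enum, then copies the array to each player state.
; AvailableColors has a RepNotify function, which is empty.
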(event Custom|SwitchOffColorEnum
  (params (ColorEnum :type Integer))
  ;[1 1 1] SwitchOffChangedColor
  (bind _output_get (Variables|Default|SetColorEnum ColorEnum))
  (Utilities|Array|SetArrayElem (Variables|Default|GetAvailableColors) _output_get false)
  (for _array_element (Variables|Default|GetPlayerArray)
    (bind _asmy_player_state (Utilities|Casting|CastToMyPlayerState _array_element))
    (Variables|/Game/Blueprints/Gameplay/MyPlayerState.MyPlayerState_C|SetAvailableColors _asmy_player_state (Variables|Default|GetAvailableColors))))

(event Custom|GrowUpCoinsAllPlayers
  ;[1 1 1] give coins to all players all the time
  (for _array_element (Variables|Default|GetPlayerArray)
    (bind _asmy_player_state (Utilities|Casting|CastToMyPlayerState _array_element))
    (Variables|/Game/Blueprints/Gameplay/MyPlayerState.MyPlayerState_C|SetCoins _asmy_player_state (+ (Variables|/Game/Blueprints/Gameplay/MyPlayerState.MyPlayerState_C|GetCoins _asmy_player_state) 1))))

(event EventBeginPlay
  ;[1 1 1] give coins to all players all the time
  (Utilities|Time|SetTimerbyEvent (delegate Custom|GrowUpCoinsAllPlayers) 2.5 true))

(fn ConstructionScript)

(fn OnRepAvailableColors)