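; Player camera pawn that moves along world X and Y from axis input and spawns buildings for the player's team.
; GetFromPCVar stores the material instance, team tag and player stats passed in, apparently from the PlayerController.
; SpawnBuilds runs only with authority, spawning the indexed class from the Builds array at the given location, owned by the pawn and rotated according to team tag.
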(event Custom|SpawnBuilds
  (params (BuildLocation :type Vector) (NumberOfBuilds :type Integer))
  ;[1 1 1] Building
  (Networking|SwitchHasAuthority
    (:Authority
      (bind _output_get (Variables|Building|SetBuildLocation BuildLocation))
      (Variables|Building|SetNumberOfBuilds NumberOfBuilds)
      (if (Utilities|Name|Equal(Name) (Variables|Default|GetTeamTag) "1")
        (Variables|Default|SetRotateBuild "0,-30.000000, 0")
        (else
          (Variables|Default|SetRotateBuild "0,90.000000, 0")))
      (Game|SpawnActorfromClass (Utilities|Array|Get(acopy) (Variables|Building|GetBuilds) (Variables|Building|GetNumberOfBuilds)) (Math|Transform|MakeTransform _output_get (Variables|Default|GetRotateBuild) "1,1,1") "Undefined" self (Game|GetInstigator)))))

(event Custom|GetFromPCVar
  (params (MaterialInstance :type Material%20Instance%20Object%20Reference) (TeamTag :type Name) (PlayerStat :type My%20Player%20State%20Object%20Reference))
  ;[1 1 1] GetVariablesFromPlayerController
  (Variables|Building|SetMaterialInstance MaterialInstance)
  (Variables|Default|SetTeamTag TeamTag)
  (Variables|Default|SetPlayerStat PlayerStat))

(event Input|AxisEvents|InputAxisMoveForward
  (params (AxisValue :type Float%20%28single-precision%29))
  ;[1 1 1] Movement
  (Pawn|Input|AddMovementInput (Math|Vector|MakeVector AxisValue 0.0 0.0) 1.0 false))

(event Input|AxisEvents|InputAxisMoveRight
  (params (AxisValue :type Float%20%28single-precision%29))
  ;[1 1 1] Movement
  (Pawn|Input|AddMovementInput (Math|Vector|MakeVector 0.0 AxisValue 0.0) 1.0 false))

(fn ConstructionScript)