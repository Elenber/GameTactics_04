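; Player controller for team-based multiplayer matches with building, handling match UI, chat, and session teardown on exit or kick.
; Team and color choice propagates to the game state, player state and camera pawn.
; Clicking traces under the cursor to select a same-team grid tile, where builds deduct coins and spawn through the pawn.
; Chat messages fan out through every PlayerState in the GameState's PlayerArray, while UpdateChat fills the gameplay widget's chat window.
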(event Custom|SendMessageToServer
  (params (Message :type Text))
  ;[1 1 1] ChatSystem
  (Variables|Chat|SetSenderText Message)
  (Variables|Chat|SetSenderName (Utilities|Text|ToText(String) (Variables|/Script/Engine.PlayerState|GetPlayerName (.AsMy%20Player%20State (Utilities|Casting|CastToMyPlayerState (Variables|GetPlayerState))))))
  (bind _asmy_game_state (Utilities|Casting|CastToMyGameState (Game|GetGameState)))
  (for _array_element (Variables|/Script/Engine.GameStateBase|GetPlayerArray _asmy_game_state)
    (bind _asmy_player_state (Utilities|Casting|CastToMyPlayerState _array_element))
    (Default|MessagetoController _asmy_player_state (Variables|Chat|GetSenderName) (Variables|Chat|GetSenderText))))

(event Custom|SetGameMode
  (params (GameMode :type Integer))
  ;[1 1 1] SetUpPlayerForNewGameMode
  (Variables|Default|SetGameMode GameMode))

(event Custom|UpdateChat
  (params (Message :type Text) (Sender :type Text))
  (bind _gameplaywb (Variables|Default|GetGamePlayWB))
  (bind _newchatwindow (Variables|/Game/UI/GameplayUI/GameplayWB.GameplayWB_C|GetNewChatWindow _gameplaywb))
  ;[1 1 1] ChatSystem
  (Utilities|IsValid _newchatwindow
    (:Is%20Valid
      (Default|AddChildtoChat _newchatwindow Message Sender))))

(event Custom|AddWBWinLose
  (params (Text :type Text))
  ;[1 1 1] AddToViewportWin/LoseWidget
  (Variables|Default|SetWinLooseText Text)
  (Viewport|RemoveAllWidgets)
  (Utilities|IsValid (Variables|Default|GetWinLoseWB)
    (:Is%20Valid
      _)
    (:Is%20Not%20Valid
      (bind _returnvalue (UserInterface|CreateWidget "/Game/UI/GameplayUI/WinLoseWB.WinLoseWB_C"))
      (Variables|Default|SetWinLoseWB _returnvalue)))
  (UserInterface|Viewport|AddtoViewport _returnvalue 0)
  (Input|SetInputModeUIOnly self (Variables|Default|GetWinLoseWB) "DoNotLock"))

(event Custom|AddGamePlayWB
  ;[1 1 1] ControllerIncludedInTheTeamWithColor
  (bind _returnvalue (UserInterface|CreateWidget "/Game/UI/GameplayUI/GameplayWB.GameplayWB_C"))
  (bind _output_get (Variables|Default|SetGamePlayWB _returnvalue))
  (UserInterface|Viewport|AddtoViewport _output_get 0)
  (Input|SetInputModeGameandUI self (Variables|Default|GetGamePlayWB) "DoNotLock" false))

(event Custom|Kick
  ;[1 1 1] ExitFromMatch
  (Game|OpenLevel(byName) "Menu")
  (|DestroySession self))

(event Custom|BuildTowerOrBarracs
  (params (PriceOfBuild :type Integer) (NumberOfBuilds :type Integer))
  ;[1 1 1] Building
  (Variables|Building|SetPriceOfBuild PriceOfBuild)
  (if (Variables|Building|GetCanBuild)
    (bind _asmy_player_state (Utilities|Casting|CastToMyPlayerState (Variables|GetPlayerState)))
    (bind _output_get (Variables|/Game/Blueprints/Gameplay/MyPlayerState.MyPlayerState_C|SetCoins _asmy_player_state (- (Variables|/Game/Blueprints/Gameplay/MyPlayerState.MyPlayerState_C|GetCoins _asmy_player_state) (Variables|Building|GetPriceOfBuild))))
    (if (>= _output_get 0)
      (Variables|Building|SetNumberOfBuilds NumberOfBuilds)
      (bind _aspawn_camera (Utilities|Casting|CastToPawnCamera (Pawn|GetControlledPawn)))
      (Variables|Building|SetCanBuild false)
      (Default|SpawnBuilds _aspawn_camera (Variables|Building|GetLocationBuild) (Variables|Building|GetNumberOfBuilds))
      (else
        (Variables|/Game/Blueprints/Gameplay/MyPlayerState.MyPlayerState_C|SetCoins _asmy_player_state (+ (Variables|/Game/Blueprints/Gameplay/MyPlayerState.MyPlayerState_C|GetCoins _asmy_player_state) (Variables|Building|GetPriceOfBuild)))))))

(event Custom|SetColorEnumAndTeam
  (params (ColorEnum :type Integer) (MaterialIsntance :type Material%20Instance%20Object%20Reference) (TeamTag :type Name))
  ;[1 1 1] ControllerIncludedInTheTeamWithColor
  (Variables|TeamLogic|SetTeamTag TeamTag)
  (Variables|TeamLogic|SetColorEnum ColorEnum)
  (Variables|Building|SetMaterialIsntance MaterialIsntance)
  (bind _asmy_game_state (Utilities|Casting|CastToMyGameState (Game|GetGameState)))
  (Default|SwitchOffColorEnum _asmy_game_state (Variables|TeamLogic|GetColorEnum))
  (bind _asmy_player_state (Utilities|Casting|CastToMyPlayerState (Variables|GetPlayerState)))
  (Variables|/Game/Blueprints/Gameplay/MyPlayerState.MyPlayerState_C|SetColorEnum _asmy_player_state (Variables|TeamLogic|GetColorEnum))
  (bind _asmy_player_state_2 (Utilities|Casting|CastToMyPlayerState (Variables|GetPlayerState)))
  (bind _aspawn_camera (Utilities|Casting|CastToPawnCamera (Pawn|GetControlledPawn)))
  (Default|GetfromPCVar _aspawn_camera (Variables|Building|GetMaterialIsntance) (Variables|TeamLogic|GetTeamTag) _asmy_player_state_2))

(event Custom|UpdateAllVariables
  (params (SelectedGrid :type My%20Grid%20Base%20Object%20Reference) (NumberOfBuilds :type Integer) (LocationBuild :type Vector) (ColorEnum :type Integer) (TeamTag :type Name))
  ;[1 1 1] Building
  (Variables|Building|SetCanBuild true)
  (Variables|Building|SetSelectedGrid SelectedGrid)
  (Variables|Building|SetNumberOfBuilds NumberOfBuilds)
  (Variables|Building|SetLocationBuild LocationBuild)
  (Variables|TeamLogic|SetTeamTag TeamTag)
  (Variables|TeamLogic|SetColorEnum ColorEnum))

(event Custom|HideLoadingScreen
  ;[1 1 1] SetUpPlayerForNewGameMode
  (bind _asmy_game_instance (Utilities|Casting|CastToMyGameInstance (Game|GetGameInstance)))
  (Default|HideLoadingScreen _asmy_game_instance))

(event Custom|CreateGameUI
  ;[1 1 1] SetUpPlayerForNewGameMode
  (bind _returnvalue (UserInterface|CreateWidget "/Game/UI/GameplayUI/TeamAndColorSelectWB.TeamAndColorSelectWB_C"))
  (bind _output_get (Variables|Default|SetSelectTeamWB _returnvalue))
  (UserInterface|Viewport|AddtoViewport _output_get 0)
  (Input|SetInputModeUIOnly self (Variables|Default|GetSelectTeamWB) "DoNotLock"))

(event EventEndPlay
  (params (EndPlayReason :type EEndPlayReason%20Enum :default "Destroyed"))
  ;[1 1 1] ExitFromMatch
  (|DestroySession self))

(event EventBeginPlay
  ;[1 1 1] SetUpPlayerForNewGameMode
  (Variables|Default|SetbShowMouseCursor true))

(event Input|KeyboardEvents|Tab
  (params (Key :type Key%20Structure))
  ;[1 1 1] ChatSystem
  (:Pressed
    (Viewport|RemoveAllWidgets)
    (bind _returnvalue (UserInterface|CreateWidget "/Game/UI/GameplayUI/TeamAndColorSelectWB.TeamAndColorSelectWB_C"))
    (bind _output_get (Variables|Default|SetSelectTeamWB _returnvalue))
    (UserInterface|Viewport|AddtoViewport _output_get 0)
    (Input|SetInputModeUIOnly self (Variables|Default|GetSelectTeamWB) "DoNotLock")))

(event Input|MouseEvents|LeftMouseButton
  (params (Key :type Key%20Structure))
  (bind _returnvalue (Game|GetPlayerController 0))
  (bind (_worldlocation _worlddirection) (Game|Player|ConvertMouseLocationToWorldSpace _returnvalue))
  ;[1 1 1] Building
  (:Pressed
    (bind (_outhit _returnvalue_2) (Collision|LineTraceForObjects _worldlocation (+ _worldlocation (* _worlddirection 2e+03)) (Utilities|Array|MakeArray "ObjectTypeQuery7") false (Utilities|Array|MakeArray self) "None"))
    (if _returnvalue_2
      (bind _outactors (Actor|GetAllActorsOfClass "/Game/Blueprints/Gameplay/Grid/MyGridBase.MyGridBase_C"))
      (for _array_element _outactors
        (Rendering|SetVisibility (Variables|/Game/Blueprints/Gameplay/Grid/MyGridBase.MyGridBase_C|GetPlane _array_element) false false))
      (bind _asmy_grid_base (Utilities|Casting|CastToMyGridBase (.HitActor (Collision|BreakHitResult _outhit))))
      (if (Utilities|Name|Equal(Name) (Variables|/Game/Blueprints/Gameplay/Grid/MyGridBase.MyGridBase_C|GetTeamTag _asmy_grid_base) (Variables|TeamLogic|GetTeamTag))
        (Variables|Building|SetLocationBuild (Variables|/Game/Blueprints/Gameplay/Grid/MyGridBase.MyGridBase_C|GetLocationGrid _asmy_grid_base))
        (CallFunction|UpdateAllVariables (Variables|Building|GetSelectedGrid) (Variables|Building|GetNumberOfBuilds) (Variables|Building|GetLocationBuild) (Variables|TeamLogic|GetColorEnum) (Variables|TeamLogic|GetTeamTag))
        (Rendering|SetVisibility (Variables|/Game/Blueprints/Gameplay/Grid/MyGridBase.MyGridBase_C|GetPlane _asmy_grid_base) true false)))))

(fn ConstructionScript)