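; Game instance that handles multiplayer lobby hosting and a loading screen widget.
; CreateLobby stores the server name, map, slots and LAN flag, creates an Advanced Session advertising name, map and LAN as extra settings, then opens the Lobby level as a listen server on success.
; JoinGame only destroys the player's current session.
; Show and hide events add and remove the loading screen through a stored widget reference.
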(event Custom|CreateLobby
  (params (ServerName :type String) (ServerMap :type String) (ServerSlots :type Integer) (ServerMethod,Lan? :type Boolean))
  (Variables|Default|SetServerName ServerName)
  (Variables|Default|SetServerMap ServerMap)
  (Variables|Default|SetServerSlots ServerSlots)
  (Variables|Default|SetServerMethod,Lan? ServerMethod,Lan?)
  (|AdvancedSession (Utilities|Array|MakeArray (Class|AdvancedSessionsLibrary|MakeLiteralSessionPropertyString "NAME" (Variables|Default|GetServerName)) (Class|AdvancedSessionsLibrary|MakeLiteralSessionPropertyString "MAP" (Variables|Default|GetServerMap)) (Class|AdvancedSessionsLibrary|MakeLiteralSessionPropertyBool "LAN" (Variables|Default|GetServerMethod,Lan?))) (Game|GetPlayerController 0) (Variables|Default|GetServerSlots) 0 (Variables|Default|GetServerMethod,Lan?) true false true true false false false true
    (:OnSuccess
      (Game|OpenLevel(byName) "Lobby" true "listen"))))

(event Custom|JoinGame
  (|DestroySession (Game|GetPlayerController 0)))

(event Custom|ShowLoadingScreen
  ;[1 1 1] LoadingScreen
  (bind _returnvalue (UserInterface|CreateWidget "/Game/UI/LobbyUI/LoadingScreenWB.LoadingScreenWB_C"))
  (bind _output_get (Variables|Default|SetLoadingWB _returnvalue))
  (UserInterface|Viewport|AddtoViewport _output_get 0))

(event Custom|HideLoadingScreen
  ;[1 1 1] LoadingScreen
  (Widget|RemovefromParent (Variables|Default|GetLoadingWB)))