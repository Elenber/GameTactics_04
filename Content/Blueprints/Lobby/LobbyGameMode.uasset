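; Lobby game mode that tracks connected players, handles chat history and kicking, and server-travels everyone into the game map.
; On login it copies server info from MyGameInstance, opens the lobby widget through LobbyPlayerController and replays the message log.
; Joins and departures broadcast server messages and rebuild every client's player list with Steam avatars and player count.
; JoinGame picks the travel map from ServerName rather than ServerMap, defaulting to Map1.
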(event Custom|JoinGame
  (bind _returnvalue (Game|GetPlayerController 0))
  ;[1 1 1] GoToGamingMap
  (if (Utilities|Enum|Equal(Enum) (Variables|Default|GetServerName) "Map1")
    (Development|ExecuteConsoleCommand "servertravel /Game/Maps/Map1" _returnvalue :!label _label)
    (elif (Utilities|Enum|Equal(Enum) (Variables|Default|GetServerName) "Map2")
      (Development|ExecuteConsoleCommand "servertravel /Game/Maps/Map2" _returnvalue)
      (else
        (goto _label))))
  (bind _asmy_game_instance (Utilities|Casting|CastToMyGameInstance (Game|GetGameInstance)))
  (Default|JoinGame _asmy_game_instance))

(event Custom|UpdateServer
  ;[1 1 1] UpdateServer
  (for _array_element (Variables|Default|GetAllPCs)
    (bind _aslobby_player_controller (Utilities|Casting|CastToLobbyPlayerController _array_element))
    (Default|ClearPlayerList _aslobby_player_controller)
    (for (_array_element_2 _array_index) (Variables|Default|GetAllPCs)
      (bind _returnvalue (Class|AdvancedSteamFriendsLibrary|GetSteamFriendAvatar (Class|AdvancedSessionsLibrary|GetUniqueNetID _array_element_2) "SteamAvatar_Small")
        (:OnSuccess
          (Variables|Default|SetFail false))
        (:AsyncLoading
          (Variables|Default|SetFail true))
        (:OnFailure
          (Variables|Default|SetFail true)))
      (Default|AddPlayer _aslobby_player_controller (Variables|Default|GetFail) (Utilities|Text|ToText(String) (Class|AdvancedSessionsLibrary|GetPlayerName _array_element_2)) _returnvalue _array_index)))
  (for _array_element_3 (Variables|Default|GetAllPCs)
    (bind _aslobby_player_controller_2 (Utilities|Casting|CastToLobbyPlayerController _array_element_3))
    (Default|UpdateNumberOfPlayer _aslobby_player_controller_2 (Utilities|Array|Length (Variables|Default|GetAllPCs)))))

(event Custom|AddMessageToChatHistory
  (params (Data :type Chat%20Messages%20Structures%20Structure))
  ;[1 1 1] Chat Logic
  ;;[1 1 1] LoadMessageHistory
  (Utilities|Array|Add (Variables|Default|GetMessageLOG) Data))

(event Custom|KickPlayer
  (params (Index :type Integer))
  ;[1 1 1] KickPlayer
  (Default|Kick (.AsLobby%20Player%20Controller (Utilities|Casting|CastToLobbyPlayerController (Utilities|Array|Get(acopy) (Variables|Default|GetAllPCs) Index)))))

(event Custom|SendServerMessage
  (params (Message :type String))
  ;[1 1 1] Chat Logic
  (bind _aslobby_player_controller (Utilities|Casting|CastToLobbyPlayerController (Game|GetPlayerController 0)))
  (Default|AddMessagefromServertoEachPlayer _aslobby_player_controller Message true (Utilities|Struct|MakeSlateColor "(R=0.000000,G=0.177542,B=1.000000,A=1.000000)")))

(event EventPostLogin
  (params (NewPlayer :type Player%20Controller%20Object%20Reference))
  ;[1 1 1] OnPostLogin Event
  (CallFunction|SendServerMessage (Utilities|String|Append (Class|AdvancedSessionsLibrary|GetPlayerName NewPlayer) " Joined"))
  (Networking|SwitchHasAuthority
    (:Authority
      (Utilities|Array|Add (Variables|Default|GetAllPCs) NewPlayer)
      (bind _asmy_game_instance (Utilities|Casting|CastToMyGameInstance (Game|GetGameInstance)))
      (Variables|Default|SetServerName (Variables|/Game/Blueprints/MyGameInstance.MyGameInstance_C|GetServerName _asmy_game_instance))
      (Variables|Default|SetServerMap (Variables|/Game/Blueprints/MyGameInstance.MyGameInstance_C|GetServerMap _asmy_game_instance))
      (Variables|Default|SetServerSlots (Variables|/Game/Blueprints/MyGameInstance.MyGameInstance_C|GetServerSlots _asmy_game_instance))
      (bind _aslobby_player_controller (Utilities|Casting|CastToLobbyPlayerController NewPlayer))
      (Default|AddLobbyWB _aslobby_player_controller (Variables|Default|GetServerName) (Variables|Default|GetServerMap) (Variables|Default|GetServerSlots))
      (CallFunction|UpdateServer)
      ;[1 1 1] Chat Logic
      ;;[1 1 1] LoadMessageHistory
      (for _array_element (Variables|Default|GetMessageLOG)
        (bind _aslobby_player_controller_2 (Utilities|Casting|CastToLobbyPlayerController NewPlayer))
        (Default|AddMessagetoChat _aslobby_player_controller_2 _array_element)))))

(event EventOnLogout
  (params (ExitingController :type Controller%20Object%20Reference))
  (bind _allpcs (Variables|Default|GetAllPCs))
  ;[1 1 1] RemovePlayerController
  (bind (_array_element _array_index) (Utilities|Array|ForEachLoopwithBreak _allpcs :!label _label)
    (:LoopBody
      (if (== ExitingController _array_element)
        (CallFunction|SendServerMessage (Utilities|String|Append (Class|AdvancedSessionsLibrary|GetPlayerName _array_element) " left"))
        (goto _label Break)))
    (:Completed
      (Utilities|Casting|CastToLobbyPlayerController (Utilities|Array|Get(acopy) _allpcs _array_index))
      (Utilities|Array|RemoveIndex (Variables|Default|GetAllPCs) _array_index)
      (CallFunction|UpdateServer))))

(fn ConstructionScript)