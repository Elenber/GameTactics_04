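; Lobby player controller that drives a player's lobby UI, chat and exit from the session.
; It creates the lobby widget, forwards player list and count updates to it, and swaps it for the GameInstance loading screen.
; Chat messages fan out through LobbyGameMode's controller list to each chat window and are saved to its history.
; Kick opens the Menu level and destroys the session, which EndPlay also destroys.
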(event Custom|AddLobbyWB
  (params (ServerName :type String) (ServerMap :type String) (ServerSlots :type Integer))
  ;[1 1 1] ShowLobbyWidget
  (Variables|Default|SetbShowMouseCursor true)
  (bind _returnvalue (UserInterface|CreateWidget "/Game/UI/LobbyUI/LobbyWB.LobbyWB_C" 0 (Utilities|Text|ToText(String) ServerName) (Utilities|Text|ToText(String) ServerMap) ServerSlots))
  (bind _output_get (Variables|Default|SetLobbyWB _returnvalue))
  (UserInterface|Viewport|AddtoViewport _output_get 1))

(event Custom|AddMessageToChat
  (params (NewParam :type Chat%20Messages%20Structures%20Structure))
  ;[1 1 1] ChatLogic
  (Default|AddChildtoChat (Variables|/Game/UI/LobbyUI/LobbyWB.LobbyWB_C|GetChatWindow (Variables|Default|GetLobbyWB)) NewParam))

(event Custom|UpdateNumberOfPlayer
  (params (CurrentPlayers :type Integer))
  ;[1 1 1] PlayerListEvents
  (Variables|/Game/UI/LobbyUI/LobbyWB.LobbyWB_C|SetCurrentPlayers (Variables|Default|GetLobbyWB) CurrentPlayers))

(event Custom|LoadingScreen
  ;[1 1 1] ShowLoadingScreen
  (Widget|RemovefromParent (Variables|Default|GetLobbyWB))
  (bind _asmy_game_instance (Utilities|Casting|CastToMyGameInstance (Game|GetGameInstance)))
  (Default|ShowLoadingScreen _asmy_game_instance))

(event Custom|ClearPlayerList
  ;[1 1 1] PlayerListEvents
  (Default|ClearPlayerList (Variables|Default|GetLobbyWB)))

(event Custom|AddPlayer
  (params (Fail? :type Boolean) (Player :type Text) (Avatar :type Texture%202D%20Object%20Reference) (PlayerIndex :type Integer))
  ;[1 1 1] PlayerListEvents
  (Default|AddPlayertoList (Variables|Default|GetLobbyWB) Fail? Player Avatar PlayerIndex))

(event Custom|Kick
  ;[1 1 1] PlayerListEvents
  (Game|OpenLevel(byName) "Menu")
  (|DestroySession self))

(event Custom|AddMessageFromServerToEachPlayer
  (params (Message :type String) (isServerMessage? :type Boolean) (Color :type Slate%20Color%20Structure))
  (bind _self self)
  (bind _playername (Class|AdvancedSessionsLibrary|GetPlayerName _self))
  (bind _chatmessagesstructures (Utilities|Struct|MakeChatMessagesStructures _playername Message Color isServerMessage?))
  ;[1 1 1] ChatLogic
  (bind _aslobby_game_mode (Utilities|Casting|CastToLobbyGameMode (Game|GetGameMode)))
  (for _array_element (Variables|/Game/Blueprints/Lobby/LobbyGameMode.LobbyGameMode_C|GetAllPCs _aslobby_game_mode)
    (bind _aslobby_player_controller (Utilities|Casting|CastToLobbyPlayerController _array_element))
    (CallFunction|AddMessagetoChat _aslobby_player_controller _chatmessagesstructures))
  (bind _aslobby_game_mode_2 (Utilities|Casting|CastToLobbyGameMode (Game|GetGameMode)))
  (Default|AddMessagetoChatHistory _aslobby_game_mode_2 _chatmessagesstructures))

(event EventEndPlay
  (params (EndPlayReason :type EEndPlayReason%20Enum :default "Destroyed"))
  ;[1 1 1] PlayerListEvents
  (|DestroySession self))

(fn ConstructionScript)